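; Game mode for a multiplayer last-player-standing match, handling player spawning, chat, deaths and session cleanup.
; It tracks swapped-in controllers, relays chat to them, and spawns selected characters at random PlayerStarts, or only destroys the pawn if one exists.
; AlguienMurio counts deaths and signals end of game to every controller once at most one player remains.
; Logout asks the Steam game instance to destroy the leaving player's session.
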(event `self.K2_OnSwapPlayerControllers`
  (params (OldPC :type "PlayerController Object Reference") (NewPC :type "PlayerController Object Reference"))
  (`KismetArrayLibrary.Array_Add` (`self.AllPlayersControllers`) NewPC))

(event `SpawnPlayer`
  (params (PlayerController :type "PlayerController Object Reference") (SelectedCharacter :type "Character Class Reference"))
  (bind _returnvalue (`Controller.K2_GetPawn` PlayerController))
  (bind _spawn_points (`self.Spawn points`))
  ;[1 1 1] Spawn the player at random player starter location
  (bind _outactors (`GameplayStatics.GetAllActorsOfClass` "/Script/Engine.PlayerStart"))
  (set `self.Spawn points` _outactors)
  (`/Engine/EditorBlueprintResources/StandardMacros.IsValid` _returnvalue
    (:`Is Valid`
      (`self.K2_DestroyActor` _returnvalue))
    (:`Is Not Valid`
      (bind _returnvalue_2 (`|SpawnActorFromClass` SelectedCharacter (`self.GetTransform` (`|GetArrayItem` _spawn_points (`KismetMathLibrary.RandomIntegerInRange` 0 (- (`KismetArrayLibrary.Array_Length` _spawn_points) 1)))) "Undefined" "OverrideRootScale" null null))
      (`Controller.Possess` PlayerController _returnvalue_2))))

(event `self.K2_OnLogout`
  (params (ExitingController :type "Controller Object Reference"))
  ;[1 1 1] On logout destroy the connected players session so they can join new games
  (bind _gameplaypc (message `/Game/Blueprints/Gameplay/BPI_GameplayPC.GameplayPCref` ExitingController))
  (bind _game_instance (message `/Game/Blueprints/BPI_GameInstance.SteamGameInstanceRef` (`GameplayStatics.GetGameInstance`)))
  (message `/Game/Blueprints/BPI_GameInstance.DestroySessionCaller` _game_instance _gameplaypc))

(event `UpdateChat`
  (params (Sender :type Text) (ChatText :type Text))
  (for _array_element (`self.AllPlayersControllers`)
    (bind _gameplaypc (message `/Game/Blueprints/Gameplay/BPI_GameplayPC.GameplayPCref` _array_element))
    (`/Game/Blueprints/Gameplay/BP_GameplayPC.UpdateChatWindow` _gameplaypc Sender ChatText)))

(event `AlguienMurio`
  (bind _output_get (set `self.Numero de personajes` (`KismetArrayLibrary.Array_Length` (`self.AllPlayersControllers`))))
  (`KismetSystemLibrary.PrintString` (`KismetStringLibrary.Conv_IntToString` _output_get))
  (set `self.Cantidad de gente muerta` (+ (`self.Cantidad de gente muerta`) 1))
  (if (>= (`self.Cantidad de gente muerta`) (- (`self.Numero de personajes`) 1))
    (`self.Fin del juego`)))

(event `self.ReceiveTick`
  (params (DeltaSeconds :type "Float (single-precision)")))

(event `Fin del juego`
  (for _array_element (`self.AllPlayersControllers`)
    (bind _gameplaypc (message `/Game/Blueprints/Gameplay/BPI_GameplayPC.GameplayPCref` _array_element))
    (`/Game/Blueprints/Gameplay/BP_GameplayPC.End of the game` _gameplaypc)))

(fn `GameplayGMref`
  (returns (GameplayGMref :type "/Game/Blueprints/Gameplay/BP_GameplayGameMode Object Reference"))
  (return self))

(fn `OnRep_Numero de personajes`)

(fn `UserConstructionScript`)